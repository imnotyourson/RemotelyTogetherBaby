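; Blueprint function library of shortcuts that return the game's core framework objects already cast to project classes.
; It fetches player 0's controller as TopDownController, the current game mode as TopDownGameMode, and a given controller's HUD as BP_HUD.
; Each function returns the cast result directly, with no handling when the cast fails.
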(fn `GetGamemode`
  (returns (`AsTop Down Game Mode` :type "/Game/Blueprints/Player/TopDownBP/TopDownGameMode Object Reference"))
  (bind _astop_down_game_mode (cast `/Game/Blueprints/Player/TopDownBP/TopDownGameMode` (`GameplayStatics.GetGameMode` null))
    (:`then`
      _)
    (:`CastFailed`
      _))
  (return _astop_down_game_mode))

(fn `GetHUD`
  (params (PlayerController :type "PlayerController Object Reference"))
  (returns (`AsBP HUD` :type "/Game/UI_UX/BP_HUD Object Reference"))
  (bind _asbp_hud (cast `/Game/UI_UX/BP_HUD` (`PlayerController.GetHUD` PlayerController))
    (:`then`
      _)
    (:`CastFailed`
      _))
  (return _asbp_hud))

(fn `GetPlayerController`
  (returns (`AsTop Down Controller` :type "/Game/Blueprints/Player/TopDownBP/TopDownController Object Reference"))
  (bind _astop_down_controller (cast `/Game/Blueprints/Player/TopDownBP/TopDownController` (`GameplayStatics.GetPlayerController` null))
    (:`then`
      _)
    (:`CastFailed`
      _))
  (return _astop_down_controller))