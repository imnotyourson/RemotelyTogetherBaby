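; Item generation Blueprint that rolls random counts of seven coloured boxes into presets for two players, apparently as an unfinished prototype.
; Space fills the P1 preset first, then overwrites P2 on later presses, printing each result.
; E and C print the P1 and P2 presets under swapped number labels.
; BeginPlay calls preset and pile-spawn events that are empty stubs, and the spawn-list merge is unconnected.
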(event `Key|E`
  (params (Key :type "Key Structure"))
  (:`Pressed`
    (`KismetSystemLibrary.PrintString` "preset 2")
    (for _array_element (`self.P1Preset`)
      (`KismetSystemLibrary.PrintString` (`KismetStringLibrary.Conv_IntToString` _array_element)))))

(event `Key|C`
  (params (Key :type "Key Structure"))
  (:`Pressed`
    (`KismetSystemLibrary.PrintString` "preset 1")
    (for _array_element (`self.P2Preset`)
      (`KismetSystemLibrary.PrintString` (`KismetStringLibrary.Conv_IntToString` _array_element)))))

(event `Spawn piles`)

(event `self.ReceiveBeginPlay`
  ;[1 1 1] start gamu
  (`self.Set presets`)
  (`self.Set presets`)
  (`self.Spawn piles`))

(event `Key|SpaceBar`
  (params (Key :type "Key Structure"))
  (bind _returnvalue (`KismetMathLibrary.RandomInteger` 5))
  ;[1 1 1] create preset
  (:`Pressed`
    (bind _output_get (set `self.BlackBox` _returnvalue))
    (bind _output_get_2 (set `self.BlueBox` _returnvalue))
    (bind _output_get_3 (set `self.GreenBox` _returnvalue))
    (bind _output_get_4 (set `self.PinkBox` _returnvalue))
    (bind _output_get_5 (set `self.RedBox` _returnvalue))
    (bind _output_get_6 (set `self.WhiteBox` _returnvalue))
    (bind _output_get_7 (set `self.YellowBox` _returnvalue))
    (if (`self.P1Done`)
      (bind _array (`|MakeArray` _output_get _output_get_2 _output_get_3 _output_get_4 _output_get_5 _output_get_6 _output_get_7))
      (bind _output_get_8 (set `self.P2Preset` _array))
      (for _array_element _output_get_8
        (`KismetSystemLibrary.PrintString` (`KismetStringLibrary.Conv_IntToString` _array_element)))
      (else
        (bind _output_get_9 (set `self.P1Preset` _array))
        (for _array_element_2 _output_get_9
          (`KismetSystemLibrary.PrintString` (`KismetStringLibrary.Conv_IntToString` _array_element_2))
          (set `self.P1Done` true))))))

(event `Set presets`
  ;[1 1 1] create preset
)

(fn `UserConstructionScript`)