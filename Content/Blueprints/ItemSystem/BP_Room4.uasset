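; BP_Room4 is a room actor that tracks placed items and scores them against required item lists for four players.
; Two recognition boxes add and remove BP_Object actors in ContentList, which StartCountingPoints converts to ints, scores and awards to players.
; Actor overlap fills HUD list texts from requirements, but every branch tests Players[0], so only the P1 branch can run, and the P3/P4 branches target ListP1.
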(event `self.ItemRecognitionBoxThingy.OnComponentBeginOverlap`
  (params (OverlappedComponent :type "PrimitiveComponent Object Reference") (OtherActor :type "Actor Object Reference") (OtherComp :type "PrimitiveComponent Object Reference") (OtherBodyIndex :type Integer) (bFromSweep :type Boolean) (SweepResult :type "HitResult Structure (by ref)"))
  (bind _asbp_object (cast `/Game/Blueprints/Objects/BP_Object` OtherActor))
  (`KismetArrayLibrary.Array_Add` (`self.ContentList`) _asbp_object))

(event `self.ItemRecognitionBoxThingy1.OnComponentBeginOverlap`
  (params (OverlappedComponent :type "PrimitiveComponent Object Reference") (OtherActor :type "Actor Object Reference") (OtherComp :type "PrimitiveComponent Object Reference") (OtherBodyIndex :type Integer) (bFromSweep :type Boolean) (SweepResult :type "HitResult Structure (by ref)"))
  (bind _asbp_object (cast `/Game/Blueprints/Objects/BP_Object` OtherActor))
  (`KismetArrayLibrary.Array_Add` (`self.ContentList`) _asbp_object))

(event `self.ItemRecognitionBoxThingy.OnComponentEndOverlap`
  (params (OverlappedComponent :type "PrimitiveComponent Object Reference") (OtherActor :type "Actor Object Reference") (OtherComp :type "PrimitiveComponent Object Reference") (OtherBodyIndex :type Integer))
  (bind _asbp_object (cast `/Game/Blueprints/Objects/BP_Object` OtherActor))
  (`KismetArrayLibrary.Array_RemoveItem` (`self.ContentList`) _asbp_object))

(event `self.ItemRecognitionBoxThingy1.OnComponentEndOverlap`
  (params (OverlappedComponent :type "PrimitiveComponent Object Reference") (OtherActor :type "Actor Object Reference") (OtherComp :type "PrimitiveComponent Object Reference") (OtherBodyIndex :type Integer))
  (bind _asbp_object (cast `/Game/Blueprints/Objects/BP_Object` OtherActor))
  (`KismetArrayLibrary.Array_RemoveItem` (`self.ContentList`) _asbp_object))

(event `StartCountingPoints`
  (`self.Set content to ints array`)
  (`self.AddPointsPerItem` null (`self.RequiredRoomItemsP1`) (`self.RequiredRoomItemsP2`) (`self.RequiredRoomItemsP3`) (`self.RequiredRoomItemsP4`))
  (`self.AddPointsToPlayers`))

(event `self.ReceiveActorBeginOverlap`
  (params (OtherActor :type "Actor Object Reference"))
  (bind _requiredroomitemsp4 (`self.RequiredRoomItemsP4`))
  (bind _requiredroomitemsp1 (`self.RequiredRoomItemsP1`))
  (bind _requiredroomitemsp2 (`self.RequiredRoomItemsP2`))
  (bind _requiredroomitemsp3 (`self.RequiredRoomItemsP3`))
  (bind _astop_down_game_mode (cast `/Game/Blueprints/Player/TopDownBP/TopDownGameMode` (`GameplayStatics.GetGameMode`)))
  (bind _asbp_hud (`/Game/Blueprints/BPFL_FunctionShortcuts.GetHUD` (`GameplayStatics.GetPlayerController` 0)))
  (bind _players (`/Game/Blueprints/Player/TopDownBP/TopDownGameMode.Players` _astop_down_game_mode))
  (if (== OtherActor (`|GetArrayItem` _players))
    (bind _returnvalue_ (`self.NewFunction_0` _requiredroomitemsp1))
    (bind _wbp_lists (`/Game/UI_UX/BP_HUD.WBP_Lists` _asbp_hud))
    (bind _listp1 (`/Game/UI_UX/Menus/WBP_Lists.ListP1` _wbp_lists))
    (set `/Game/UI_UX/Menus/WBP_IndividualList.Text_0` _returnvalue_ _listp1)
    (bind _returnvalue__2 (`self.NewFunction_0` _requiredroomitemsp1 1))
    (set `/Game/UI_UX/Menus/WBP_IndividualList.Text_1` _returnvalue__2 _listp1)
    (bind _returnvalue__3 (`self.NewFunction_0` _requiredroomitemsp1 2))
    (set `/Game/UI_UX/Menus/WBP_IndividualList.Text_2` _returnvalue__3 _listp1)
    (bind _returnvalue__4 (`self.NewFunction_0` _requiredroomitemsp1 3))
    (set `/Game/UI_UX/Menus/WBP_IndividualList.Text_3` _returnvalue__4 _listp1)
    (elif (== OtherActor (`|GetArrayItem` _players))
      (bind _returnvalue__5 (`self.NewFunction_0` _requiredroomitemsp2))
      (bind _listp2 (`/Game/UI_UX/Menus/WBP_Lists.ListP2` _wbp_lists))
      (set `/Game/UI_UX/Menus/WBP_IndividualList.Text_0` _returnvalue__5 _listp2)
      (bind _returnvalue__6 (`self.NewFunction_0` _requiredroomitemsp2 1))
      (set `/Game/UI_UX/Menus/WBP_IndividualList.Text_1` _returnvalue__6 _listp2)
      (bind _returnvalue__7 (`self.NewFunction_0` _requiredroomitemsp2 2))
      (set `/Game/UI_UX/Menus/WBP_IndividualList.Text_2` _returnvalue__7 _listp2)
      (bind _returnvalue__8 (`self.NewFunction_0` _requiredroomitemsp2 3))
      (set `/Game/UI_UX/Menus/WBP_IndividualList.Text_3` _returnvalue__8 _listp2)
      (elif (== OtherActor (`|GetArrayItem` _players))
        (bind _returnvalue__9 (`self.NewFunction_0` _requiredroomitemsp3))
        (bind _listp1_2 (`/Game/UI_UX/Menus/WBP_Lists.ListP1` _wbp_lists))
        (set `/Game/UI_UX/Menus/WBP_IndividualList.Text_0` _returnvalue__9 _listp1_2)
        (bind _returnvalue__10 (`self.NewFunction_0` _requiredroomitemsp3 1))
        (set `/Game/UI_UX/Menus/WBP_IndividualList.Text_1` _returnvalue__10 _listp1_2)
        (bind _returnvalue__11 (`self.NewFunction_0` _requiredroomitemsp3 2))
        (set `/Game/UI_UX/Menus/WBP_IndividualList.Text_2` _returnvalue__11 _listp1_2)
        (bind _returnvalue__12 (`self.NewFunction_0` _requiredroomitemsp3 3))
        (set `/Game/UI_UX/Menus/WBP_IndividualList.Text_3` _returnvalue__12 _listp1_2)
        (elif (== OtherActor (`|GetArrayItem` _players))
          (bind _returnvalue__13 (`self.NewFunction_0` _requiredroomitemsp4))
          (bind _listp1_3 (`/Game/UI_UX/Menus/WBP_Lists.ListP1` _wbp_lists))
          (set `/Game/UI_UX/Menus/WBP_IndividualList.Text_0` _returnvalue__13 _listp1_3)
          (bind _returnvalue__14 (`self.NewFunction_0` _requiredroomitemsp4 1))
          (set `/Game/UI_UX/Menus/WBP_IndividualList.Text_1` _returnvalue__14 _listp1_3)
          (bind _returnvalue__15 (`self.NewFunction_0` _requiredroomitemsp4 2))
          (set `/Game/UI_UX/Menus/WBP_IndividualList.Text_2` _returnvalue__15 _listp1_3)
          (bind _returnvalue__16 (`self.NewFunction_0` _requiredroomitemsp4 3))
          (set `/Game/UI_UX/Menus/WBP_IndividualList.Text_3` _returnvalue__16 _listp1_3))))))

(fn `UserConstructionScript`
  (`parent.UserConstructionScript`))