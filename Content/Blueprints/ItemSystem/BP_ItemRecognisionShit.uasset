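; BP_ItemRecognisionShit is an item-recognition actor that tallies interior items by tag for two-player scoring.
; Start gathers all InteriorItemsReference actors, removes same-name entries, and counts first-tag matches against ItemTags into ItemIndexArray.
; AddPointsPerItem compares a room's counts with player arrays, adding 100 per match, though its inverted P2 zero check blocks Player 2 points.
; Calculatepoints loops over instances with an empty body; the scoring calls are disconnected.
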(event `Start`
  (bind _item_array (`self.Item array`))
  (bind _itemindexarray (`self.ItemIndexArray`))
  (bind _outactors (`GameplayStatics.GetAllActorsOfClass` (`self.Interior_items_reference`)))
  (bind _output_get (set `self.Item array` _outactors))
  (bind _returnvalue (`KismetArrayLibrary.Array_Length` _output_get))
  (for _index (range (+ _returnvalue 1))
    (for _index_2 (range (+ (`KismetArrayLibrary.Array_Length` _item_array) 1))
      (if (== _index_2 _index)
        _
        (elif (`KismetStringLibrary.EqualEqual_StrStr` (`KismetSystemLibrary.GetObjectName` (`|GetArrayItem` _item_array _index)) (`KismetSystemLibrary.GetObjectName` (`|GetArrayItem` (`self.Item array`) _index_2)))
          (`KismetArrayLibrary.Array_Remove` (`self.Item array`) _index_2)))))
  (for _index_3 (range (+ _returnvalue 1))
    (for _index_4 (range (+ (`KismetArrayLibrary.Array_Length` (`self.ItemTags`)) 1))
      (if (== (`|GetArrayItem` (`Actor.Tags` (`|GetArrayItem` (`self.Item array`) _index_3))) (`|GetArrayItem` (`self.ItemTags`) _index_4))
        (bind _result (`/Engine/EditorBlueprintResources/StandardMacros.IncrementInt` (`|GetArrayItem` _itemindexarray _index_4))
          (:`  `
            (`KismetArrayLibrary.Array_Set` _itemindexarray _index_4 _result)))))))

(event `Calculate points`
  (bind _outactors (`GameplayStatics.GetAllActorsOfClass` "BP_ItemRecognisionShit_C"))
  (for _ _outactors
    _))

(fn `AddPointsPerItem`
  (params (Room :type "/Game/Blueprints/ItemSystem/BP_ItemRecognisionShit Object Reference") (P1 :type "Array of Integer") (P2 :type "Array of Integer"))
  (bind _itemindexarray (`/Game/Blueprints/ItemSystem/BP_ItemRecognisionShit.ItemIndexArray` Room))
  (for _index (range (+ (`KismetArrayLibrary.Array_Length` _itemindexarray) 1))
    (bind _output (`|GetArrayItem` _itemindexarray _index))
    (if (not (== _output 0))
      (bind _output_2 (`|GetArrayItem` P1 _index))
      (if (not (== _output_2 0))
        (while (not (or (== (`self.itemamountcalc`) _output) (== (`self.itemamountcalc`) _output_2)))
          (`/Engine/EditorBlueprintResources/StandardMacros.IncrementInt` (`self.itemamountcalc`)
            (:`  `
              (set `self.Player 1 points` (+ (`self.Player 1 points`) 100)))))
        (set `self.itemamountcalc` 0))
      (bind _output_3 (`|GetArrayItem` P2 _index))
      (if (== _output_3 0)
        (while (not (or (== (`self.itemamountcalc`) _output) (== (`self.itemamountcalc`) _output_3)))
          (`/Engine/EditorBlueprintResources/StandardMacros.IncrementInt` (`self.itemamountcalc`)
            (:`  `
              (set `self.Player 2 points` (+ (`self.Player 2 points`) 100)))))
        (else
          (set `self.itemamountcalc` 0))))))

(fn `UserConstructionScript`)