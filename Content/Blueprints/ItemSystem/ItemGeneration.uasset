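; Item generator that spawns random piles of colored boxes for two players, P1 and P2.
; Each Space press rolls a count per box color, saves it as that player's preset and prints it for debugging.
; The first press triggers P1Pile and later presses trigger P2Pile, both spawning boxes at SpawnTransform.
; SetPresets, called on BeginPlay, is an empty stub.
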(event `P1Pile`
  (bind _spawntransform (`self.spawnTransform`))
  ;[1 1 1] Spawn sheet
  (`KismetSystemLibrary.PrintString` "p1")
  (`|ExecutionSequence`
    (:`then_0`
      (for _ (range 1 (+ (`self.BlackBox`) 1))
        (`|SpawnActorFromClass` "/Game/Blueprints/Objects/BP_BlackBox.BP_BlackBox_C" _spawntransform "AlwaysSpawn" "OverrideRootScale" null null)))
    (:`then_1`
      (for _ (range 1 (+ (`self.BlueBox`) 1))
        (`|SpawnActorFromClass` "/Game/Blueprints/Objects/BP_BB.BP_BB_C" _spawntransform "AlwaysSpawn" "OverrideRootScale" null null)))
    (:`then_2`
      (for _ (range 1 (+ (`self.GreenBox`) 1))
        (`|SpawnActorFromClass` "/Game/Blueprints/Objects/BP_GreenBox.BP_GreenBox_C" _spawntransform "AlwaysSpawn" "OverrideRootScale" null null)))
    (:`then_3`
      (for _ (range 1 (+ (`self.PinkBox`) 1))
        (`|SpawnActorFromClass` "/Game/Blueprints/Objects/BP_PB.BP_PB_C" _spawntransform "AlwaysSpawn" "OverrideRootScale" null null)))
    (:`then_4`
      (for _ (range 1 (+ (`self.RedBox`) 1))
        (`|SpawnActorFromClass` "/Game/Blueprints/Objects/BP_RedBox.BP_RedBox_C" _spawntransform "AlwaysSpawn" "OverrideRootScale" null null)))
    (:`then_5`
      (for _ (range 1 (+ (`self.WhiteBox`) 1))
        (`|SpawnActorFromClass` "/Game/Blueprints/Objects/BP_WhiteBox.BP_WhiteBox_C" _spawntransform "AlwaysSpawn" "OverrideRootScale" null null)))
    (:`then_6`
      (for _ (range 1 (+ (`self.YellowBox`) 1))
        (`|SpawnActorFromClass` "/Game/Blueprints/Objects/BP_YB.BP_YB_C" _spawntransform "AlwaysSpawn" "OverrideRootScale" null null)))))

(event `P2Pile`
  (bind _spawntransform (`self.spawnTransform`))
  ;[1 1 1] Spawn sheet
  (`KismetSystemLibrary.PrintString` "p2")
  (`|ExecutionSequence`
    (:`then_0`
      (for _ (range 1 (+ (`self.BlackBox`) 1))
        (`|SpawnActorFromClass` "/Game/Blueprints/Objects/BP_BlackBox.BP_BlackBox_C" _spawntransform "AlwaysSpawn" "OverrideRootScale" null null)))
    (:`then_1`
      (for _ (range 1 (+ (`self.BlueBox`) 1))
        (`|SpawnActorFromClass` "/Game/Blueprints/Objects/BP_BB.BP_BB_C" _spawntransform "AlwaysSpawn" "OverrideRootScale" null null)))
    (:`then_2`
      (for _ (range 1 (+ (`self.GreenBox`) 1))
        (`|SpawnActorFromClass` "/Game/Blueprints/Objects/BP_GreenBox.BP_GreenBox_C" _spawntransform "AlwaysSpawn" "OverrideRootScale" null null)))
    (:`then_3`
      (for _ (range 1 (+ (`self.PinkBox`) 1))
        (`|SpawnActorFromClass` "/Game/Blueprints/Objects/BP_PB.BP_PB_C" _spawntransform "AlwaysSpawn" "OverrideRootScale" null null)))
    (:`then_4`
      (for _ (range 1 (+ (`self.RedBox`) 1))
        (`|SpawnActorFromClass` "/Game/Blueprints/Objects/BP_RedBox.BP_RedBox_C" _spawntransform "AlwaysSpawn" "OverrideRootScale" null null)))
    (:`then_5`
      (for _ (range 1 (+ (`self.WhiteBox`) 1))
        (`|SpawnActorFromClass` "/Game/Blueprints/Objects/BP_WhiteBox.BP_WhiteBox_C" _spawntransform "AlwaysSpawn" "OverrideRootScale" null null)))
    (:`then_6`
      (for _ (range 1 (+ (`self.YellowBox`) 1))
        (`|SpawnActorFromClass` "/Game/Blueprints/Objects/BP_YB.BP_YB_C" _spawntransform "AlwaysSpawn" "OverrideRootScale" null null)))))

(event `Key|M`
  (params (Key :type "Key Structure")))

(event `self.ReceiveBeginPlay`
  ;[1 1 1] start gamu
  (`self.Set presets`)
  (`self.Set presets`))

(event `Key|SpaceBar`
  (params (Key :type "Key Structure"))
  (bind _returnvalue (`KismetMathLibrary.RandomInteger` 5))
  ;[1 1 1] create preset
  (:`Pressed`
    (bind _output_get (set `self.BlackBox` _returnvalue))
    (bind _output_get_2 (set `self.BlueBox` _returnvalue))
    (bind _output_get_3 (set `self.GreenBox` _returnvalue))
    (bind _output_get_4 (set `self.PinkBox` _returnvalue))
    (bind _output_get_5 (set `self.RedBox` _returnvalue))
    (bind _output_get_6 (set `self.WhiteBox` _returnvalue))
    (bind _output_get_7 (set `self.YellowBox` _returnvalue))
    (if (`self.P1Done`)
      (bind _array (`|MakeArray` _output_get _output_get_2 _output_get_3 _output_get_4 _output_get_5 _output_get_6 _output_get_7))
      (bind _output_get_8 (set `self.P2Preset` _array))
      (`|ExecutionSequence`
        (:`then_0`
          (`self.P2Pile`))
        (:`then_1`
          (for _array_element _output_get_8
            (`KismetSystemLibrary.PrintString` (`KismetStringLibrary.Conv_IntToString` _array_element)))))
      (else
        (bind _output_get_9 (set `self.P1Preset` _array))
        (`|ExecutionSequence`
          (:`then_0`
            (`self.P1Pile`)
            (set `self.P1Done` true))
          (:`then_1`
            (for _array_element_2 _output_get_9
              (`KismetSystemLibrary.PrintString` (`KismetStringLibrary.Conv_IntToString` _array_element_2)))))))))

(event `Set presets`
  ;[1 1 1] create preset
)

(fn `UserConstructionScript`)